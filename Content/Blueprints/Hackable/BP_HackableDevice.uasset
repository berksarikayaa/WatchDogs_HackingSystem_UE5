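; BP_HackableDevice is a hackable world actor that the player triggers with E to play an alert sound and emit AI-audible noise as a distraction.
; A looping timer runs CheckHackingRange, which requires the player within HackingDistance, the device near screen center via projected position, and recently rendered.
; Passing shows the widget and enables input on the actor; failing reverses both.
; Pressing E briefly hides the widget before MakeNoise fires after a retriggerable delay.
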(event `self.ReceiveBeginPlay`
  (`KismetSystemLibrary.K2_SetTimer` null "CheckHackingRange" 0.6 true))

(event `Key|E`
  (params (Key :type "Key Structure"))
  (:`Pressed`
    (`GameplayStatics.PlaySoundAtLocation` "/Game/Blueprints/Hackable/Alert.Alert" (`self.K2_GetActorLocation`) (struct) 1.0 1.0 0.0 null null null null)
    (`SceneComponent.SetHiddenInGame` (`self.Widget`) true false)
    (`KismetSystemLibrary.RetriggerableDelay` 1.0)
    (`SceneComponent.SetHiddenInGame` (`self.Widget`) false false)
    (`self.MakeNoise` 1.0 (`GameplayStatics.GetPlayerPawn` 0) (`self.K2_GetActorLocation`) 2000.0)))

(fn `CheckHackingRange`
  (bind _returnvalue (`WidgetLayoutLibrary.GetViewportSize`))
  (bind (_returnvalue_x _returnvalue_y) (`KismetMathLibrary.BreakVector2D` (/ (`KismetMathLibrary.GetAbs2D` (- (/ _returnvalue (2.0 2.0)) (`GameplayStatics.ProjectWorldToScreen` (`GameplayStatics.GetPlayerController` 0) (`self.K2_GetActorLocation`)))) _returnvalue)))
  (if (< (`self.GetDistanceTo` (`GameplayStatics.GetPlayerPawn` 0)) (`self.HackingDistance`))
    (if (and (< _returnvalue_x 0.2) (< _returnvalue_y 0.4) (`self.WasRecentlyRendered` 0.2))
      (`SceneComponent.SetVisibility` (`self.Widget`) true false)
      (`self.EnableInput` (`GameplayStatics.GetPlayerController` 0))
      (else
        (`SceneComponent.SetVisibility` (`self.Widget`) false false :!label _label)
        (`self.DisableInput` (`GameplayStatics.GetPlayerController` 0))))
    (else
      (goto _label))))

(fn `UserConstructionScript`)